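; Mailbox actor that shows a completion indicator on first overlap and an "already completed" indicator on later ones.
; Both components start hidden on BeginPlay, and any actor overlap briefly reveals the relevant one.
; The Complete component is destroyed after its two-second display, so its validity serves as the completion flag.
; AlreadyCompleted is simply hidden again after the same delay, so it can repeat.
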(event `self.ReceiveBeginPlay`
  (`SceneComponent.SetVisibility` (`self.Complete`) false false)
  (`SceneComponent.SetVisibility` (`self.AlreadyCompleted`) false false))

(event `self.ReceiveActorBeginOverlap`
  (params (OtherActor :type "Actor Object Reference"))
  (if (`KismetSystemLibrary.IsValid` (`self.Complete`))
    (`SceneComponent.SetVisibility` (`self.Complete`) true false)
    (`KismetSystemLibrary.Delay` 2.0)
    (`ActorComponent.K2_DestroyComponent` (`self.Complete`))
    (else
      (`SceneComponent.SetVisibility` (`self.AlreadyCompleted`) true false)
      (`KismetSystemLibrary.Delay` 2.0)
      (`SceneComponent.SetVisibility` (`self.AlreadyCompleted`) false false))))

(fn `UserConstructionScript`)